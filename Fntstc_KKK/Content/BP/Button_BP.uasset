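; Interactable button actor that moves a referenced actor, apparently a car, along a spline.
; Box overlap with the ThirdPersonCharacter toggles input and a gate so Interact only triggers the button nearby.
; Pressing runs the button timeline, whose update starts a second timeline setting the actor's location from spline time; releasing plays a sound.
; The button lerp has identical zero endpoints, and spline rotation is left unconnected.
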(event OnComponentBeginOverlap(Box)
  (params (OverlappedComponent :type Primitive%20Component%20Object%20Reference) (OtherActor :type Actor%20Object%20Reference) (OtherComp :type Primitive%20Component%20Object%20Reference) (OtherBodyIndex :type Integer) (bFromSweep :type Boolean) (SweepResult :type Hit%20Result%20Structure%20%28by%20ref%29))
  (Utilities|Casting|CastToThirdPersonCharacter OtherActor)
  (Input|EnableInput (Game|GetPlayerController 0))
  (Utilities|FlowControl|Gate true) ; enters at Open
)

(event OnComponentEndOverlap(Box)
  (params (OverlappedComponent :type Primitive%20Component%20Object%20Reference) (OtherActor :type Actor%20Object%20Reference) (OtherComp :type Primitive%20Component%20Object%20Reference) (OtherBodyIndex :type Integer))
  (Utilities|Casting|CastToThirdPersonCharacter OtherActor)
  (Input|DisableInput (Game|GetPlayerController 0))
  (Utilities|FlowControl|Gate true) ; enters at Close
)

(event Input|ActionEvents|InputActionInteract
  (params (Key :type Key%20Structure :default "None"))
  (:Pressed
    (Utilities|FlowControl|Gate true
      (:Exit
        ;[1 1 1] Button Anim
        (bind _newtrack_0 (Timeline|Button%20Press Play)
          (:Update
            (Transformation|SetRelativeLocation (Variables|Default|GetButton) (Math|Vector|Lerp(Vector) "0, 0, 0" "0, 0, 0" _newtrack_0) false false)
            ;[1 1 1] Move Car
            (bind _spline_time (Timeline|Time_Move_1Car Play)
              (:Update
                (Transformation|SetActorTransform (Variables|Default|GetActorToAnim) (Math|Transform|MakeTransform (Spline|GetLocationatTime (Variables|/Game/BP/Spline_1.Spline_1_C|GetSpline (Variables|Default|GetSpline)) _spline_time "World" false) "0, 0, 0" "1,1,1")))))))))
  (:Released
    (Audio|PlaySoundatLocation "/Game/Sound/fernando-f1-v12_cut.fernando-f1-v12_cut" (Transformation|GetActorLocation) "0, 0, 0" 1.0 1.0 0.0 0 0 0)))

(fn ConstructionScript)